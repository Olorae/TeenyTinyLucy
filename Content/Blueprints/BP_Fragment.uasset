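; BP_Fragment is a spinning fragment actor that plays an attached sound until the third-person character overlaps it.
; BeginPlay attaches the scintillement sound to the box component with fragment attenuation and starts a fast looping timer by function name, apparently targeting Rotate.
; Rotate adds a small local yaw to the static mesh on each call.
; Overlap with BP_ThirdPersonCharacter only stops the sound, with no collection or destroy logic here.
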(event EventBeginPlay
  (bind _returnvalue (Audio|SpawnSoundAttached "/Game/SFX/SC_Scintillement.SC_Scintillement" (Variables|Default|GetBoxComponent) "None" "0, 0, 0" "0, 0, 0" "KeepRelativeOffset" false 1.0 1.0 0.0 "/Game/SFX/SoundAttenuation/SA_Fragment.SA_Fragment" 0 false))
  (Variables|Default|SetScintillementSound _returnvalue)
  (Utilities|Time|SetTimerbyFunctionName 0 (Variables|Default|GetRotateFuntionName) 0.005 true))

(event Collision|EventActorBeginOverlap
  (params (OtherActor :type Actor%20Object%20Reference))
  (Utilities|Casting|CastToBP_ThirdPersonCharacter OtherActor)
  (Audio|Components|Audio|Stop (Variables|Default|GetScintillementSound)))

(fn ConstructionScript)

(fn Rotate
  (Transformation|AddLocalRotation (Variables|Default|GetStaticMeshComponent) (Math|Rotator|MakeRotator 0.0 0.0 0.5) false false))