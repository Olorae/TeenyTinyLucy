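; BP_BrickStructure is a structure of Lego brick meshes that collapses when the player or companion touches it.
; On actor overlap it casts the other actor to BP_ThirdPersonCharacter, then to BP_Companion if that fails.
; A match on either prints a debug "Hello" and loops over the brick components to enable physics simulation on each.
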(event EventBeginPlay)

(event Collision|EventActorBeginOverlap
  (params (OtherActor :type Actor%20Object%20Reference))
  (Utilities|Casting|CastToBP_ThirdPersonCharacter OtherActor
    (:then
      _)
    (:CastFailed
      (Utilities|Casting|CastToBP_Companion OtherActor)))
  (Development|PrintString "Hello")
  (for _array_element (Utilities|Array|MakeArray (Variables|Default|GetSM_LegoBrick) (Variables|Default|GetSM_LegoBrick1) (Variables|Default|GetSM_LegoBrick2) (Variables|Default|GetSM_LegoBrick3) (Variables|Default|GetSM_LegoBrick4) (Variables|Default|GetSM_LegoBrick5) (Variables|Default|GetSM_LegoBrick6) (Variables|Default|GetSM_LegoBrick7) (Variables|Default|GetSM_LegoBrick8) (Variables|Default|GetSM_LegoBrick18) (Variables|Default|GetSM_LegoBrick10) (Variables|Default|GetSM_LegoBrick11) (Variables|Default|GetSM_LegoBrick19) (Variables|Default|GetSM_LegoBrick20) (Variables|Default|GetSM_LegoBrick21) (Variables|Default|GetSM_LegoBrick22) (Variables|Default|GetSM_LegoBrick9) (Variables|Default|GetSM_LegoBrick12) (Variables|Default|GetSM_LegoBrick13) (Variables|Default|GetSM_LegoBrick14) (Variables|Default|GetSM_LegoBrick15) (Variables|Default|GetSM_LegoBrick16) (Variables|Default|GetSM_LegoBrick17))
    (Physics|SetSimulatePhysics _array_element true)))

(fn ConstructionScript)